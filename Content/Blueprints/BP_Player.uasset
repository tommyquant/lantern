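; RTS-style player pawn that pans and zooms the camera and turns mouse clicks into firefly selection and orders through GameManager.
; Axis input and screen-edge checks pan the pawn, zoom clamps spring arm length, and a timeline lerps it to focus locations.
; Holding left click past a delay drag-selects via a HUD rectangle and a spawned BP_DragSelect box fitted between ground traces.
; Right click messages IClickable actors or moves selected fireflies on Landscape.
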(event `self.ReceiveBeginPlay`
  (bind _returnvalue (`|SpawnActorFromClass` "/Game/Blueprints/BP_DragSelect.BP_DragSelect_C" (`KismetMathLibrary.MakeTransform` (0.0 0.0 0.0)) "Undefined" "OverrideRootScale" null null))
  (set `self.DragSelector` _returnvalue))

(event `self.ReceiveTick`
  (params (DeltaSeconds :type "Float (single-precision)"))
  (`self.CheckScroll`)
  (`self.UpdateDragSelect`))

(event `InputAxis|ScrollUp`
  (params (AxisValue :type "Float (single-precision)"))
  (`self.K2_AddActorLocalOffset` (`KismetMathLibrary.MakeVector` (* AxisValue (* (`self.ScrollSpeed`) (`GameplayStatics.GetWorldDeltaSeconds`)))) true))

(event `InputAxis|ScrollRight`
  (params (AxisValue :type "Float (single-precision)"))
  (`self.K2_AddActorLocalOffset` (`KismetMathLibrary.MakeVector` 0.0 (* AxisValue (* (`self.ScrollSpeed`) (`GameplayStatics.GetWorldDeltaSeconds`)))) true))

(event `InputAxis|Zoom`
  (params (AxisValue :type "Float (single-precision)"))
  (`self.Zoom` (+ (`SpringArmComponent.TargetArmLength` (`self.SpringArm`)) (* AxisValue (* (`self.ZoomSpeed`) (`GameplayStatics.GetWorldDeltaSeconds`))))))

(event `InputAction|LeftClick`
  (params (Key :type "Key Structure"))
  (:`Pressed`
    (`self.SetInitialDragSelect`))
  (:`Released`
    (`|ExecutionSequence`
      (:`then_0`
        (if (`self.DragSelectEnabled`)
          (`/Game/Blueprints/BP_GameManager.SelectFireflies` (`self.GameManager`) (`/Game/Blueprints/BP_DragSelect.Fireflies` (`self.DragSelector`)))
          (else
            (bind _hitactor (`self.TraceMouse` false)
              (:`HitClickableActor`
                (bind _asbp_firefly (cast `/Game/Blueprints/BP_Firefly` _hitactor)
                  (:`then`
                    (`/Game/Blueprints/BP_GameManager.SelectFireflies` (`self.GameManager`) (`|MakeArray` _asbp_firefly)))
                  (:`CastFailed`
                    (`/Game/Blueprints/BP_GameManager.SelectFireflies` (`self.GameManager`) (`|MakeArray` null :!type "/Game/Blueprints/BP_Firefly Object Reference") :!label _label))))
              (:`HitNonClickableActor`
                (goto _label))
              (:`NoHit`
                (goto _label))))))
      (:`then_1`
        (`self.DisableDragSelect`)))))

(event `InputAction|RightClick`
  (params (Key :type "Key Structure"))
  (bind _gamemanager (`self.GameManager`))
  (:`Pressed`
    (bind (_hitactor _hitresult) (`self.TraceMouse` false)
      (:`HitClickableActor`
        (message `/Game/Blueprints/IClickable.OnRightClick` _hitactor _gamemanager))
      (:`HitNonClickableActor`
        (bind (_bblockinghit _binitialoverlap _time _distance _location _impactpoint _normal _impactnormal _physmat _hitactor_2) (`GameplayStatics.BreakHitResult` _hitresult))
        (cast `Landscape` _hitactor_2)
        (`/Game/Blueprints/BP_GameManager.MoveFireflies` _gamemanager _location)
        (for _array_element (`/Game/Blueprints/BP_GameManager.SelectedFireflies` _gamemanager)
          (set `/Game/Blueprints/BP_Firefly.TargetLantern` null _array_element))))))

(event `FocusOnLocation`
  (params (CurrentLocation :type "Vector Structure") (TargetLocation :type "Vector Structure"))
  (bind (_direction _alpha) (`Timeline|CameraTimeline` :!via `PlayFromStart`)
    (:`Update`
      (`self.K2_SetActorLocation` (`KismetMathLibrary.VLerp` CurrentLocation TargetLocation _alpha)))))

(fn `CheckScroll`
  (locals (MousePos :type "Vector2D Structure") (ScrollSpeedDelta :type "Float (double-precision)"))
  (bind _returnvalue_x (`KismetMathLibrary.BreakVector2D` (`WidgetLayoutLibrary.GetViewportSize`)))
  (bind (_returnvalue_x_2 _returnvalue_y) (`KismetMathLibrary.BreakVector2D` (`WidgetLayoutLibrary.GetViewportSize`)))
  (bind (_mousepos_x _mousepos_y) (`KismetMathLibrary.BreakVector2D` (`local.MousePos`)))
  (bind _mousepos_x_2 (`KismetMathLibrary.BreakVector2D` (`local.MousePos`)))
  (bind _mousepos_x_3 (`KismetMathLibrary.BreakVector2D` (`local.MousePos`)))
  (bind (_mousepos_x_4 _mousepos_y_2) (`KismetMathLibrary.BreakVector2D` (`local.MousePos`)))
  (set `local.ScrollSpeedDelta` (* (`self.ScrollSpeed`) (`GameplayStatics.GetWorldDeltaSeconds`)))
  (bind _returnvalue (`WidgetLayoutLibrary.GetMousePositionOnViewport`))
  (set `local.MousePos` (* _returnvalue (`WidgetLayoutLibrary.GetViewportScale`)))
  (`|ExecutionSequence`
    (:`then_0`
      (if (< _mousepos_x_2 (`self.EdgeScrollThickness`))
        (`self.K2_AddActorLocalOffset` (`KismetMathLibrary.MakeVector` 0.0 (* (`local.ScrollSpeedDelta`) -1.0)) true)))
    (:`then_1`
      (if (> _mousepos_x_3 (- _returnvalue_x (`self.EdgeScrollThickness`)))
        (`self.K2_AddActorLocalOffset` (`KismetMathLibrary.MakeVector` 0.0 (`local.ScrollSpeedDelta`)) true)))
    (:`then_2`
      (if (< _mousepos_y (`self.EdgeScrollThickness`))
        (`self.K2_AddActorLocalOffset` (`KismetMathLibrary.MakeVector` (`local.ScrollSpeedDelta`)) true)))
    (:`then_3`
      (if (> _mousepos_y_2 (- _returnvalue_y (`self.EdgeScrollThickness`)))
        (`self.K2_AddActorLocalOffset` (`KismetMathLibrary.MakeVector` (* (`local.ScrollSpeedDelta`) -1.0)) true)))))

(fn `DisableDragSelect`
  (bind _box (`/Game/Blueprints/BP_DragSelect.Box` (`self.DragSelector`)))
  (set `self.DragSelectTimer` 0.0)
  (set `self.DragSelectTimerEnabled` false)
  (bind _hud (`self.GetHUD`)
    (:`Success`
      (set `/Game/Blueprints/Base/HUD_Game.DrawDragSelect` false _hud)
      (`BoxComponent.SetBoxExtent` _box (0.0 0.0 0.0) true)
      (`PrimitiveComponent.SetCollisionEnabled` _box "NoCollision")
      (set `self.DragSelectEnabled` false)
      (`KismetArrayLibrary.Array_Clear` (`/Game/Blueprints/BP_DragSelect.Fireflies` (`self.DragSelector`))))))

(fn `SetInitialDragSelect`
  (bind _dragselector (`self.DragSelector`))
  (bind (_locationx _locationy) (`PlayerController.GetMousePosition` (`GameplayStatics.GetPlayerController` 0)))
  (`|ExecutionSequence`
    (:`then_0`
      (bind _hud (`self.GetHUD`)
        (:`Success`
          (bind _output_get (set `/Game/Blueprints/Base/HUD_Game.InitialPosition` (`KismetMathLibrary.MakeVector2D` _locationx _locationy) _hud))
          (set `self.InitialMouseScreenSpace` _output_get))))
    (:`then_1`
      (set `self.DragSelectTimerEnabled` true)
      (`PrimitiveComponent.SetCollisionEnabled` (`/Game/Blueprints/BP_DragSelect.Box` _dragselector) "QueryOnly")
      (`KismetArrayLibrary.Array_Clear` (`/Game/Blueprints/BP_DragSelect.Fireflies` _dragselector)))))

(fn `UpdateDragSelect`
  (bind (_locationx _locationy) (`PlayerController.GetMousePosition` (`GameplayStatics.GetPlayerController` 0)))
  (bind (_returnvalue_x _returnvalue_y) (`KismetMathLibrary.BreakVector2D` (/ (+ (`self.InitialMouseWorldSpace`) (`self.CurrentMouseWorldSpace`)) 2.0)))
  (bind (_returnvalue_x_2 _returnvalue_y_2) (`KismetMathLibrary.BreakVector2D` (/ (- (`self.CurrentMouseWorldSpace`) (`self.InitialMouseWorldSpace`)) 2.0)))
  (`|ExecutionSequence`
    (:`then_0`
      (bind _hud (`self.GetHUD`)
        (:`Success`
          (set `/Game/Blueprints/Base/HUD_Game.CurrentPosition` (`KismetMathLibrary.MakeVector2D` _locationx _locationy) _hud)
          (bind (_location_x _location_y) (`self.TraceMouseSimple` false)
            (:`Out`
              (set `self.CurrentMouseWorldSpace` (`KismetMathLibrary.MakeVector2D` _location_x _location_y))
              (bind (_location_x_2 _location_y_2) (`self.TraceMouseSimple` true)
                (:`Out`
                  (set `self.InitialMouseWorldSpace` (`KismetMathLibrary.MakeVector2D` _location_x_2 _location_y_2)))))))))
    (:`then_1`
      (if (`self.DragSelectTimerEnabled`)
        (bind _output_get (set `self.DragSelectTimer` (+ (`self.DragSelectTimer`) (`GameplayStatics.GetWorldDeltaSeconds`))))
        (if (>= _output_get (`self.DragSelectMinTime`))
          (set `self.DragSelectEnabled` true)
          (bind _hud_2 (`self.GetHUD`)
            (:`Success`
              (set `/Game/Blueprints/Base/HUD_Game.DrawDragSelect` true _hud_2)
              (`self.K2_SetActorLocation` (`self.DragSelector`) (`KismetMathLibrary.MakeVector` _returnvalue_x _returnvalue_y) false false)
              (`BoxComponent.SetBoxExtent` (`/Game/Blueprints/BP_DragSelect.Box` (`self.DragSelector`)) (`KismetMathLibrary.MakeVector` (`KismetMathLibrary.Abs` _returnvalue_x_2) (`KismetMathLibrary.Abs` _returnvalue_y_2) 200.0) true))))))))

(fn `UserConstructionScript`)

(fn `Zoom`
  (params (NewZoom :type "Float (double-precision)"))
  (bind _maxzoom (`self.MaxZoom`))
  (set `SpringArmComponent.TargetArmLength` (`KismetMathLibrary.SelectFloat` (`self.MinZoom`) (`KismetMathLibrary.SelectFloat` _maxzoom NewZoom (> NewZoom _maxzoom)) (< NewZoom (`self.MinZoom`))) (`self.SpringArm`)))
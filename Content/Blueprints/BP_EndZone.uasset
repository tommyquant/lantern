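; Level goal zone that is completed when fireflies matching every required color are inside its sphere.
; On BeginPlay it converts any assigned light source, resumes music from the GameInstance's saved time, and builds the HUD with a widget per required color.
; Sphere overlaps assign or release non-light-source fireflies in color slots, then recheck completion.
; Completion shows the next-level button, activates particles and fades up the plant's emissive dynamic material via a timeline.
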(event `self.ReceiveBeginPlay`
  (bind _lightsource (`self.LightSource`))
  (`|ExecutionSequence`
    (:`then_0`
      (`/Engine/EditorBlueprintResources/StandardMacros.IsValid` _lightsource
        (:`Is Valid`
          (`/Game/Blueprints/BP_Firefly.ConvertToLight` _lightsource false false))))
    (:`then_1`
      (bind _returnvalue (`|CreateWidget` "/Game/UI/WBP_HUD.WBP_HUD_C" null self))
      (bind _output_get (set `self.HUDWidget` _returnvalue))
      (`UserWidget.AddToViewport` _output_get 0)
      (bind _returnvalue_2 (`KismetMaterialLibrary.CreateDynamicMaterialInstance` "/Game/Materials/MI_GiantPlant.MI_GiantPlant"))
      (bind _output_get_2 (set `self.PlantMaterial` _returnvalue_2))
      (`PrimitiveComponent.SetMaterial` (`self.Plant`) 0 _output_get_2)
      (bind _asgi_game (cast `/Game/Blueprints/Base/GI_Game` (`GameplayStatics.GetGameInstance`)))
      (`AudioComponent.Play` (`self.Music`) (`/Game/Blueprints/Base/GI_Game.MusicTime` _asgi_game)))
    (:`then_2`
      (for _index (range (`KismetArrayLibrary.Array_Length` (`self.RequiredColors`)))
        (bind _returnvalue_3 (`|CreateWidget` "/Game/UI/WBP_Required.WBP_Required_C" null self _index))
        (setmembers `/Game/Blueprints/SRequiredColor` :`StructRef` (`|GetArrayItem` (`self.RequiredColors`) _index) :`RequiredWidget` _returnvalue_3)
        (`/Game/UI/WBP_Required.Initialize` _returnvalue_3)
        (`PanelWidget.AddChild` (`/Game/UI/WBP_HUD.RequiredBox` (`self.HUDWidget`)) _returnvalue_3)))))

(event `self.ReceiveTick`
  (params (DeltaSeconds :type "Float (single-precision)"))
  (`SceneComponent.K2_AddWorldRotation` (`self.Ring`) (`KismetMathLibrary.MakeRotator` 0.0 0.0 (* DeltaSeconds (`self.RotationRate`))) false false))

(event `self.Sphere.OnComponentBeginOverlap`
  (params (OverlappedComponent :type "PrimitiveComponent Object Reference") (OtherActor :type "Actor Object Reference") (OtherComp :type "PrimitiveComponent Object Reference") (OtherBodyIndex :type Integer) (bFromSweep :type Boolean) (SweepResult :type "HitResult Structure (by ref)"))
  (bind _asbp_firefly (cast `/Game/Blueprints/BP_Firefly` OtherActor))
  (if (not (`/Game/Blueprints/BP_Firefly.IsLightSource` _asbp_firefly))
    (`self.AddFirefly` _asbp_firefly)
    (`self.CheckRequiredFireflies` :!label _label)))

(event `self.Sphere.OnComponentEndOverlap`
  (params (OverlappedComponent :type "PrimitiveComponent Object Reference") (OtherActor :type "Actor Object Reference") (OtherComp :type "PrimitiveComponent Object Reference") (OtherBodyIndex :type Integer))
  (bind _asbp_firefly (cast `/Game/Blueprints/BP_Firefly` OtherActor))
  (if (not (`/Game/Blueprints/BP_Firefly.IsLightSource` _asbp_firefly))
    (`self.RemoveFirefly` _asbp_firefly)
    (goto _label)))

(event `AnimatePlantMaterial`
  (params (Active :type Boolean))
  (if Active
    (bind (_direction _alpha) (`Timeline|PlantTimeline` :!label _label_2)
      (:`Update`
        (`MaterialInstanceDynamic.SetScalarParameterValue` (`self.PlantMaterial`) "EmissiveStrength" (`KismetMathLibrary.Lerp` 0.0 3.0 _alpha))))
    (else
      (goto _label_2 :!via `Reverse`))))

(event `self.Music.OnAudioPlaybackPercent`
  (params (PlayingSoundWave :type "SoundWave Object Reference") (PlaybackPercent :type "Float (single-precision)"))
  (set `self.MusicTime` (* (`SoundBase.Duration` PlayingSoundWave) PlaybackPercent)))

(event `InputAction|ShowMenu`
  (params (Key :type "Key Structure"))
  (:`Pressed`
    (`/Game/UI/WBP_HUD.ToggleMenu` (`self.HUDWidget`))))

(fn `AddFirefly`
  (params (FireflyToAdd :type "/Game/Blueprints/BP_Firefly Object Reference"))
  (bind _fireflytoadd (`local.FireflyToAdd`))
  (for _index (range (`KismetArrayLibrary.Array_Length` (`self.RequiredColors`)))
    (bind _output (`|GetArrayItem` (`self.RequiredColors`) _index))
    (bind (_color _firefly) (break `/Game/Blueprints/SRequiredColor` _output))
    (`/Engine/EditorBlueprintResources/StandardMacros.IsValid` _firefly
      (:`Is Not Valid`
        (if (`|EnumEquality` _color (`/Game/Blueprints/BP_Firefly.LightColor` (`local.FireflyToAdd`)))
          (`|ExecutionSequence`
            (:`then_0`
              (setmembers `/Game/Blueprints/SRequiredColor` :`StructRef` _output :`Firefly` _fireflytoadd)
              (set `/Game/Blueprints/BP_Firefly.RequiredColorIndex` _index _fireflytoadd)
              (`/Game/UI/WBP_Required.FillCircle` (`.RequiredWidget_8_E9C8F52D40B53991F6AC25BEFBE8BF2E` (break `/Game/Blueprints/SRequiredColor` _output)) true))
            (:`then_1`
              (break))))))))

(fn `CheckRequiredFireflies`
  (locals (Success :type Boolean :default true))
  (bind _hudwidget (`self.HUDWidget`))
  (bind _particles (`self.Particles`))
  (for _array_element (`self.RequiredColors`)
    (`/Engine/EditorBlueprintResources/StandardMacros.IsValid` (`.Firefly_5_A1A9DF244BB046B73B0139B646711236` (break `/Game/Blueprints/SRequiredColor` _array_element))
      (:`Is Not Valid`
        (set `local.Success` false))))
  (if (`local.Success`)
    (if (not (`self.NextLevelButtonVisible`))
      (`/Game/UI/WBP_HUD.SetNextLevelButtonVisibility` _hudwidget true)
      (`ActorComponent.Activate` _particles false)
      (`self.AnimatePlantMaterial` true)
      (set `self.NextLevelButtonVisible` true))
    (else
      (`/Game/UI/WBP_HUD.SetNextLevelButtonVisibility` _hudwidget false)
      (`ActorComponent.Deactivate` _particles)
      (`self.AnimatePlantMaterial` false)
      (set `self.NextLevelButtonVisible` false))))

(fn `RemoveFirefly`
  (params (FireflyToRemove :type "/Game/Blueprints/BP_Firefly Object Reference"))
  (bind _output (`|GetArrayItem` (`self.RequiredColors`) (`/Game/Blueprints/BP_Firefly.RequiredColorIndex` FireflyToRemove)))
  (if (== (`.Firefly_5_A1A9DF244BB046B73B0139B646711236` (break `/Game/Blueprints/SRequiredColor` _output)) (`local.FireflyToRemove`))
    (bind _structout (setmembers `/Game/Blueprints/SRequiredColor` :`StructRef` _output :`Firefly` null))
    (`/Game/UI/WBP_Required.FillCircle` (`.RequiredWidget_8_E9C8F52D40B53991F6AC25BEFBE8BF2E` (break `/Game/Blueprints/SRequiredColor` _structout)) false)))

(fn `UserConstructionScript`
  (`SphereComponent.SetSphereRadius` (`self.Sphere`) (`self.Radius`) true))
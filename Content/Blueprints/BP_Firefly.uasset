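; Selectable, color-coded firefly that moves by AI and loses health whenever no compatible light source touches it.
; Light sources register themselves on overlapping fireflies of matching or wildcard color, which restores full health; health drives particle alpha.
; ConvertToLight turns it into a stationary lantern, with timelines scaling light and collision radius together; at zero health this is temporary and fades out.
; Hover and selection drive a dynamic outline material.
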(event `self.ReceiveBeginPlay`
  (bind _returnvalue (`KismetMaterialLibrary.CreateDynamicMaterialInstance` "/Game/Materials/MI_SelectionOutline.MI_SelectionOutline"))
  (bind _output_get (set `self.SelectionMaterial` _returnvalue))
  (`PrimitiveComponent.SetMaterial` (`self.SelectionOutline`) 0 _output_get)
  (`self.AdjustSelectionMaterial` 0.0 true)
  (set `self.Health` (`self.MaxHealth`)))

(event `self.ReceiveTick`
  (params (DeltaSeconds :type "Float (single-precision)"))
  (if (`self.IsLightSource`)
    _
    (elif (== (`KismetArrayLibrary.Array_Length` (`self.LightSourcesTouching`)) 0)
      (`self.SetHealth` (`self.HealthMinusDamage`))
      (else
        (`self.SetHealth` (`self.MaxHealth`))))))

(event `self.LightSourceCollision.OnComponentBeginOverlap`
  (params (OverlappedComponent :type "PrimitiveComponent Object Reference") (OtherActor :type "Actor Object Reference") (OtherComp :type "PrimitiveComponent Object Reference") (OtherBodyIndex :type Integer) (bFromSweep :type Boolean) (SweepResult :type "HitResult Structure (by ref)"))
  (bind _lightcolor (`self.LightColor`))
  (bind _asbp_firefly (cast `/Game/Blueprints/BP_Firefly` OtherActor))
  (bind _lightcolor_2 (`/Game/Blueprints/BP_Firefly.LightColor` _asbp_firefly))
  (if (or (`|EnumEquality` _lightcolor_2 _lightcolor) (`|EnumEquality` _lightcolor_2 "NewEnumerator0") (`|EnumEquality` _lightcolor "NewEnumerator0"))
    (`KismetArrayLibrary.Array_AddUnique` (`/Game/Blueprints/BP_Firefly.LightSourcesTouching` _asbp_firefly) self)))

(event `self.CapsuleComponent.OnBeginCursorOver`
  (params (TouchedComponent :type "PrimitiveComponent Object Reference"))
  (if (not (`self.IsSelected`))
    (`self.AdjustSelectionMaterial` 1.0 true (struct :`A` 1.0))))

(event `self.CapsuleComponent.OnEndCursorOver`
  (params (TouchedComponent :type "PrimitiveComponent Object Reference"))
  (if (not (`self.IsSelected`))
    (`self.AdjustSelectionMaterial` 0.0 true)))

(event `self.LightSourceCollision.OnComponentEndOverlap`
  (params (OverlappedComponent :type "PrimitiveComponent Object Reference") (OtherActor :type "Actor Object Reference") (OtherComp :type "PrimitiveComponent Object Reference") (OtherBodyIndex :type Integer))
  (bind _asbp_firefly (cast `/Game/Blueprints/BP_Firefly` OtherActor))
  (`KismetArrayLibrary.Array_RemoveItem` (`/Game/Blueprints/BP_Firefly.LightSourcesTouching` _asbp_firefly) self))

(event `/Game/Blueprints/IClickable.OnLeftClick`
  (params (GameManager :type "/Game/Blueprints/BP_GameManager Object Reference"))
  (`/Game/Blueprints/BP_GameManager.SelectFirefly` GameManager self))

(event `MoveToLocation`
  (params (Location :type "Vector Structure"))
  (if (not (`self.IsLightSource`))
    (`|AIMoveTo` self Location)))

(event `ConvertToLight`
  (params (IsTemporary :type Boolean) (PlaySound :type Boolean))
  (`|ExecutionSequence`
    (:`then_0`
      (`PrimitiveComponent.SetCollisionEnabled` (`self.CapsuleComponent`) "NoCollision")
      (`PrimitiveComponent.SetCollisionEnabled` (`self.LightSourceCollision`) "QueryOnly")
      (`SceneComponent.SetVisibility` (`self.PointLight`) true false)
      (`SceneComponent.SetVisibility` (`self.SelectionOutline`) false false)
      (`ParticleSystemComponent.SetTemplate` (`self.Fireflies`) "/Game/Particles/Firefly/PS_FireflyLantern.PS_FireflyLantern")
      (`self.SetActorTickEnabled` false)
      (set `self.IsLightSource` true)
      (`|ExecutionSequence`
        (:`then_0`
          (if PlaySound
            (`GameplayStatics.PlaySound2D` "/Game/Audio/SFX_LanternOn.SFX_LanternOn")))
        (:`then_1`
          (if (> (`self.Health`) 0.0)
            (`self.SetHealth` (`self.MaxHealth`))))))
    (:`then_1`
      (bind (_direction _alpha) (`Timeline|EnableLightTimeline` :!via `PlayFromStart`)
        (:`Update`
          (`self.AdjustLightRadius` _alpha))
        (:`Finished`
          (if IsTemporary
            (`self.FadeLight`)))))))

(event `FadeLight`
  (`TimelineComponent.SetPlayRate` (`self.DisableLightTimeline`) (/ 1.0 (`self.DyingLightDuration`)))
  (bind (_direction _alpha) (`Timeline|DisableLightTimeline` :!via `PlayFromStart`)
    (:`Update`
      (`self.AdjustLightRadius` _alpha))
    (:`Finished`
      (`PrimitiveComponent.SetCollisionEnabled` (`self.LightSourceCollision`) "NoCollision")
      (`SceneComponent.SetVisibility` (`self.PointLight`) false false))))

(fn `AdjustLightRadius`
  (params (Alpha :type "Float (double-precision)"))
  (bind _lightradius (`self.LightRadius`))
  (`CapsuleComponent.SetCapsuleRadius` (`self.LightSourceCollision`) (`KismetMathLibrary.Lerp` 0.0 _lightradius Alpha) true)
  (`PointLightComponent.SetAttenuationRadius` (`self.PointLight`) (`KismetMathLibrary.Lerp` 0.0 (* _lightradius (`self.LightSourceMultiplier`)) Alpha)))

(fn `AdjustSelectionMaterial`
  (params (NewOpacity :type "Float (double-precision)") (ChangeOpacity :type Boolean) (NewColor :type "LinearColor Structure") (ChangeColor :type Boolean))
  (`|ExecutionSequence`
    (:`then_0`
      (if (`local.ChangeOpacity`)
        (`MaterialInstanceDynamic.SetScalarParameterValue` (`self.SelectionMaterial`) "Opacity" (`local.NewOpacity`))))
    (:`then_1`
      (if (`local.ChangeColor`)
        (`MaterialInstanceDynamic.SetVectorParameterValue` (`self.SelectionMaterial`) "Color" (`local.NewColor`))))))

(fn `SetHealth`
  (params (SetHealth :type "Float (double-precision)"))
  (set `self.Health` SetHealth)
  (`|ExecutionSequence`
    (:`then_0`
      (if (<= (`self.Health`) 0.0)
        (set `self.Health` 0.0)
        (`self.ConvertToLight` true true)))
    (:`then_1`
      (`ParticleSystemComponent.SetFloatParameter` (`self.Fireflies`) "Alpha" (`self.HealthPercentage`)))))

(fn `SetSelected`
  (params (IsSelected :type Boolean))
  (if IsSelected
    (`self.AdjustSelectionMaterial` 1.0 true (`/Game/Blueprints/BPL_Colors.GetColor` (`self.LightColor`)) true)
    (set `self.IsSelected` true)
    (else
      (`self.AdjustSelectionMaterial` 0.0 true (struct :`R` 1.0 :`G` 1.0 :`B` 1.0 :`A` 1.0) true)
      (set `self.IsSelected` false))))

(fn `UserConstructionScript`
  (bind _lightradius (`self.LightRadius`))
  (bind _pointlight (`self.PointLight`))
  (`ParticleSystemComponent.SetVectorParameter` (`self.Fireflies`) "InitialColor" (`KismetMathLibrary.Conv_LinearColorToVector` (`/Game/Blueprints/BPL_Colors.GetColor` (`self.LightColor`))))
  (`CapsuleComponent.SetCapsuleRadius` (`self.LightSourceCollision`) _lightradius true)
  (`PointLightComponent.SetAttenuationRadius` _pointlight (* _lightradius (`self.LightSourceMultiplier`)))
  (`LightComponent.SetLightColor` _pointlight (`/Game/Blueprints/BPL_Colors.GetColor` (`self.LightColor`)) true)
  (if (`self.IsLightSource`)
    (`SceneComponent.SetVisibility` (`self.PointLight`) true false)
    (`SceneComponent.SetVisibility` (`self.SelectionOutline`) false true)))
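; Spline-driven fence actor that builds fence runs along an editable spline in the construction script.
; Each pair of neighboring points gets a spline mesh bent by their local locations and tangents, using one of four fence meshes.
; Mesh choice is unseeded random, so the variants can change whenever construction reruns.
; A single static mesh component is added at the spline's end, indexed by the point count.
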(fn `UserConstructionScript`
  (bind _spline (`self.Spline`))
  (bind _returnvalue (`SplineComponent.GetNumberOfSplinePoints` (`self.Spline`)))
  (for _index (range (+ (- _returnvalue 2) 1))
    (bind _returnvalue_2 (`AddComponent|NODE_AddSplineMeshComponent-0`))
    (`StaticMeshComponent.SetStaticMesh` _returnvalue_2 (select `int` (`KismetMathLibrary.RandomIntegerInRange` 0 3) :`0` "/Game/Meshes/SM_Fence_01.SM_Fence_01" :`1` "/Game/Meshes/SM_Fence_02.SM_Fence_02" :`2` "/Game/Meshes/SM_Fence_03.SM_Fence_03" :`3` "/Game/Meshes/SM_Fence_04.SM_Fence_04" :!type "StaticMesh Object Reference"))
    (bind (_location _tangent) (`SplineComponent.GetLocationAndTangentAtSplinePoint` _spline _index "Local"))
    (bind (_location_2 _tangent_2) (`SplineComponent.GetLocationAndTangentAtSplinePoint` _spline (+ _index 1) "Local"))
    (`SplineMeshComponent.SetStartAndEnd` _returnvalue_2 _location _tangent _location_2 _tangent_2 true))
  (`AddComponent|NODE_AddStaticMeshComponent-0` :`RelativeTransform` (`KismetMathLibrary.MakeTransform` (`SplineComponent.GetLocationAtSplinePoint` (`self.Spline`) (- _returnvalue 0) "Local"))))
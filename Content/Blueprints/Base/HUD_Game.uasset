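; HUD_Game is the game's HUD Blueprint, which draws a rectangular drag-selection box on screen.
; DrawHUD checks the DrawDragSelect flag and, when set, draws four lines between InitialPosition and CurrentPosition using a configurable color and thickness.
; EnableDragSelect toggles that flag, while the graph itself never updates the two corner positions.
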(event `self.ReceiveBeginPlay`)

(event `self.ReceiveDrawHUD`
  (params (SizeX :type Integer) (SizeY :type Integer))
  (bind (_initialposition_x _initialposition_y) (`KismetMathLibrary.BreakVector2D` (`self.InitialPosition`)))
  (bind _currentposition_x (`KismetMathLibrary.BreakVector2D` (`self.CurrentPosition`)))
  (bind _initialposition_x_2 (`KismetMathLibrary.BreakVector2D` (`self.InitialPosition`)))
  (bind (_currentposition_x_2 _currentposition_y) (`KismetMathLibrary.BreakVector2D` (`self.CurrentPosition`)))
  (bind (_initialposition_x_3 _initialposition_y_2) (`KismetMathLibrary.BreakVector2D` (`self.InitialPosition`)))
  (bind (_currentposition_x_3 _currentposition_y_2) (`KismetMathLibrary.BreakVector2D` (`self.CurrentPosition`)))
  (bind (_initialposition_x_4 _initialposition_y_3) (`KismetMathLibrary.BreakVector2D` (`self.InitialPosition`)))
  (bind (_currentposition_x_4 _currentposition_y_3) (`KismetMathLibrary.BreakVector2D` (`self.CurrentPosition`)))
  (if (`self.DrawDragSelect`)
    (`self.DrawLine` _initialposition_x _initialposition_y _currentposition_x _initialposition_y (`self.LineColor`) (`self.LineThickness`))
    (`self.DrawLine` _initialposition_x_3 _initialposition_y_2 _initialposition_x_3 _currentposition_y_2 (`self.LineColor`) (`self.LineThickness`))
    (`self.DrawLine` _currentposition_x_4 _initialposition_y_3 _currentposition_x_4 _currentposition_y_3 (`self.LineColor`) (`self.LineThickness`))
    (`self.DrawLine` _initialposition_x_2 _currentposition_y _currentposition_x_2 _currentposition_y (`self.LineColor`) (`self.LineThickness`))))

(fn `EnableDragSelect`
  (params (Enable :type Boolean))
  (set `self.DrawDragSelect` Enable))

(fn `UserConstructionScript`)
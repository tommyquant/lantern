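; BP_GameManager handles selection and move orders for fireflies in an RTS-like control scheme.
; On BeginPlay it registers itself with BP_Player and spawns a BP_MoveCircle marker.
; SelectFireflies clears the previous selection's state, then marks and stores the new group.
; MoveFireflies activates the marker and sends a lone firefly to the target, or spreads groups around it using index-based angular offsets rotated by each firefly's look-at direction.
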(event `self.ReceiveBeginPlay`
  (bind _asbp_player (cast `/Game/Blueprints/BP_Player` (`GameplayStatics.GetPlayerPawn` 0)))
  (bind _output_get (set `self.Player` _asbp_player))
  (set `/Game/Blueprints/BP_Player.GameManager` self _output_get)
  (bind _returnvalue (`|SpawnActorFromClass` "/Game/Blueprints/BP_MoveCircle.BP_MoveCircle_C" (`KismetMathLibrary.MakeTransform` (0.0 0.0 0.0) (struct) (0.0 0.0 0.0)) "Undefined" "OverrideRootScale" null null))
  (set `self.MoveCircle` _returnvalue))

(fn `MoveFireflies`
  (params (Location :type "Vector Structure"))
  (bind _selectedfireflies (`self.SelectedFireflies`))
  (bind _returnvalue (`KismetArrayLibrary.Array_Length` _selectedfireflies))
  (`/Game/Blueprints/BP_MoveCircle.Activate` (`self.MoveCircle`) Location)
  (for (_array_element _array_index) _selectedfireflies
    (if (> _returnvalue 1)
      (`/Game/Blueprints/BP_Firefly.MoveToLocation` _array_element (+ (* (`KismetMathLibrary.GreaterGreater_VectorRotator` (`KismetMathLibrary.GetRightVector` (`KismetMathLibrary.MakeRotator` 0.0 0.0 (`KismetMathLibrary.Conv_IntToDouble` (* _array_index (/ 360 _returnvalue))))) (`KismetMathLibrary.FindLookAtRotation` (`self.K2_GetActorLocation` _array_element) Location)) 75.0) Location))
      (else
        (`/Game/Blueprints/BP_Firefly.MoveToLocation` _array_element Location)))))

(fn `SelectFireflies`
  (params (NewFireflies :type "Array of /Game/Blueprints/BP_Firefly Object Reference"))
  (`|ExecutionSequence`
    (:`then_0`
      (for _array_element (`self.SelectedFireflies`)
        (`/Engine/EditorBlueprintResources/StandardMacros.IsValid` _array_element
          (:`Is Valid`
            (`/Game/Blueprints/BP_Firefly.SetSelected` _array_element false)))))
    (:`then_1`
      (for _array_element_2 NewFireflies
        (`/Engine/EditorBlueprintResources/StandardMacros.IsValid` _array_element_2
          (:`Is Valid`
            (`/Game/Blueprints/BP_Firefly.SetSelected` _array_element_2 true)))))
    (:`then_2`
      (set `self.SelectedFireflies` NewFireflies))))

(fn `UserConstructionScript`)
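; BP_MoveCircle is an actor that shows an animated circle marker on a plane at a requested location, apparently as movement feedback.
; On BeginPlay it creates a dynamic instance of MI_MoveCircle and applies it to the plane.
; Activate moves the actor to the given X and Y at a fixed height, then restarts a timeline that drives its scale and material opacity.
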(event `self.ReceiveBeginPlay`
  (bind _returnvalue (`KismetMaterialLibrary.CreateDynamicMaterialInstance` "/Game/Materials/MI_MoveCircle.MI_MoveCircle"))
  (bind _output_get (set `self.Material` _returnvalue))
  (`PrimitiveComponent.SetMaterial` (`self.Plane`) 0 _output_get))

(event `Activate`
  (params (Location :type "Vector Structure"))
  (`self.K2_SetActorLocation` (`KismetMathLibrary.MakeVector` Location_X Location_Y 10.0))
  (bind (_direction _scalealpha _opacity) (`Timeline|AnimationTimeline` :!via `PlayFromStart`)
    (:`Update`
      (`self.SetActorScale3D` (`KismetMathLibrary.Conv_DoubleToVector` (`KismetMathLibrary.Lerp` 0.0 1.5 _scalealpha)))
      (`MaterialInstanceDynamic.SetScalarParameterValue` (`self.Material`) "Opacity" _opacity))))

(fn `UserConstructionScript`)